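; BP_PowerUpBase is a base Blueprint for power-ups that the player triggers by overlapping its Collider.
; The first overlap by a BP_PlayerCharacter, gated by DoOnce, calls PowerUp on that character, plays a sound and prints PowerUpName.
; BeginPlay fills in a default name if none is set.
; ApplyEffect is a placeholder that only prints a message and is not called in this graph.
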(event `self.ReceiveBeginPlay`
  (if (`KismetStringLibrary.IsEmpty` (`self.PowerUpName`))
    (set `self.PowerUpName` "DefaultPower") ; DefaultName
  ))

(event `self.Collider.OnComponentBeginOverlap`
  (params (OverlappedComponent :type "PrimitiveComponent Object Reference") (OtherActor :type "Actor Object Reference") (OtherComp :type "PrimitiveComponent Object Reference") (OtherBodyIndex :type Integer) (bFromSweep :type Boolean) (SweepResult :type "HitResult Structure (by ref)"))
  (bind _asbp_player_character (cast `/Game/Dynamics/PlayerCharacter/Blueprints/BP_PlayerCharacter` OtherActor))
  (`/Engine/EditorBlueprintResources/StandardMacros.DoOnce` false
    (:`Completed`
      (`/Game/Dynamics/PlayerCharacter/Blueprints/BP_PlayerCharacter.PowerUp` _asbp_player_character null)
      (`GameplayStatics.PlaySound2D` "/Engine/VREditor/Sounds/UI/Camera_Shutter.Camera_Shutter" 1.0 1.0 0.0 null null)
      (`KismetSystemLibrary.PrintString` (`self.PowerUpName`)))))

(event `ApplyEffect`
  (params (Target :type "/Game/Dynamics/PlayerCharacter/Blueprints/BP_PlayerCharacter Object Reference"))
  (`KismetSystemLibrary.PrintString` "Base Powerup"))

(fn `UserConstructionScript`)