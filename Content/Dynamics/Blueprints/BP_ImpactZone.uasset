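; BP_ImpactZone is an actor that shows a warning circle decal, presumably marking an incoming impact.
; BeginPlay gives the decal a dynamic material instance so its FadeAmount parameter can be driven at runtime.
; FadeIn and FadeOut play one timeline forward or in reverse, and the actor destroys itself when it finishes at zero alpha.
; Tick grows the decal by a fixed step each frame, independent of delta time.
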(event `FadeIn`
  ;[1 1 1] Fade In/Out Timeline
  (`TimelineComponent.SetPlaybackPosition` (`self.FadeTimeline`) 0.0 false true)
  (bind (_direction _alpha) (`Timeline|FadeTimeline` :!label _label)
    (:`Update`
      (`MaterialInstanceDynamic.SetScalarParameterValue` (`self.ImpactDecalMat`) "FadeAmount" _alpha))
    (:`Finished`
      (if (<= _alpha 0.0)
        (`self.K2_DestroyActor`)))))

(event `self.ReceiveTick`
  (params (DeltaSeconds :type "Float (single-precision)"))
  ;[1 1 1] Scale up over time
  (`SceneComponent.SetWorldScale3D` (`self.DecalWarningCircle`) (- (`SceneComponent.K2_GetComponentScale` (`self.DecalWarningCircle`)) (-0.03 -0.03 -0.03))))

(event `FadeOut`
  ;[1 1 1] Fade In/Out Timeline
  (`TimelineComponent.SetPlaybackPosition` (`self.FadeTimeline`) 1.0 false true)
  (goto _label :!via `Reverse`))

(event `self.ReceiveBeginPlay`
  ;[1 1 1] Set Material (So it can be edited by blueprints)
  (bind _returnvalue (`KismetMaterialLibrary.CreateDynamicMaterialInstance` "/Game/Statics/OtherMaterials/M_DecalMat.M_DecalMat"))
  (bind _output_get (set `self.ImpactDecalMat` _returnvalue))
  (`DecalComponent.SetDecalMaterial` (`self.DecalWarningCircle`) _output_get))

(fn `UserConstructionScript`)