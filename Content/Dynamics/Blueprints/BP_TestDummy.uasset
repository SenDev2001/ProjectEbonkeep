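; BP_TestDummy is a damageable character that serves as a test target and dies when its health runs out.
; It fills CurrentHealth to MaxHealth on BeginPlay, and AnyDamage subtracts from it with clamping while spawning an explosion effect at the actor on each hit.
; At zero health, OnDeath blocks further damage, disables movement, ragdolls the mesh through physics simulation and destroys the actor after a short delay.
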(event `InitHealth`
  ;[0.1916 1 0] Init Health
  (set `self.CurrentHealth` (`self.MaxHealth`)))

(event `self.ReceiveBeginPlay`
  ;[0 0.5735 1] Begin Play
  (`parent.ReceiveBeginPlay`)
  (`self.InitHealth`))

(event `self.ReceiveAnyDamage`
  (params (Damage :type "Float (single-precision)") (DamageType :type "DamageType Object Reference") (InstigatedBy :type "Controller Object Reference") (DamageCauser :type "Actor Object Reference"))
  ;[1 0.3896 0] On take damage, check if dead, remove hp, update health UI, trigger death if dead
  (if (not (`self.IsDead`))
    (set `self.CurrentHealth` (`KismetMathLibrary.FClamp` (- (`self.CurrentHealth`) Damage) 0.0 (`self.MaxHealth`)))
    (`GameplayStatics.SpawnEmitterAtLocation` "/Game/Statics/StarterContent/Particles/P_Explosion.P_Explosion" (`self.K2_GetActorLocation`))
    (if (== (`self.CurrentHealth`) 0.0)
      (`self.OnDeath`))))

(event `OnDeath`
  ;[1 0.001672 0] On Death
  (set `self.IsDead` true)
  (`CharacterMovementComponent.DisableMovement` (`self.CharacterMovement`))
  (`PrimitiveComponent.SetSimulatePhysics` (`self.Mesh`) true)
  (`KismetSystemLibrary.Delay` 3.0)
  (`self.K2_DestroyActor`))

(fn `UserConstructionScript`
  (`parent.UserConstructionScript`))