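; BP_Meteor is a meteor hazard that damages the player on overlap and explodes on impact.
; On BeginPlay a downward trace spawns a BP_ImpactZone on the surface below and fades it in as a warning marker.
; Hits count only after a Tick-driven timer's arming delay, triggering particles, camera shake and random-pitch sound, then fading the marker and destroying the meteor.
; A longer timeout removes meteors that fail to explode.
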(event `self.Collider.OnComponentBeginOverlap`
  (params (OverlappedComponent :type "PrimitiveComponent Object Reference") (OtherActor :type "Actor Object Reference") (OtherComp :type "PrimitiveComponent Object Reference") (OtherBodyIndex :type Integer) (bFromSweep :type Boolean) (SweepResult :type "HitResult Structure (by ref)"))
  ;[1 1 1] Overlap, Damage Entity
  (if (== OtherActor (`GameplayStatics.GetPlayerCharacter` 0))
    (`GameplayStatics.ApplyDamage` OtherActor 50.0)))

(event `self.Sphere.OnComponentHit`
  (params (HitComponent :type "PrimitiveComponent Object Reference") (OtherActor :type "Actor Object Reference") (OtherComp :type "PrimitiveComponent Object Reference") (NormalImpulse :type "Vector Structure") (Hit :type "HitResult Structure (by ref)"))
  (bind _returnvalue (`SceneComponent.K2_GetComponentLocation` (`self.Sphere`)))
  ;[1 1 1] Spawn explosion on hit
  (if (and (!= HitComponent (`self.sun`)) (!= HitComponent (`self.Collider`)))
    (if (>= (`self.Timer`) 5.0)
      (`GameplayStatics.SpawnEmitterAtLocation` "/Game/Statics/StarterContent/Particles/P_Explosion.P_Explosion" _returnvalue (struct) (8.0 8.0 8.0))
      (`GameplayStatics.PlayWorldCameraShake` "/Game/Dynamics/BossFight/BP_MeteorCameraShake.BP_MeteorCameraShake_C" _returnvalue 0.0 8000.0 1.2 true)
      (`GameplayStatics.PlaySoundAtLocation` "/Game/Statics/SFX/Meteor_Hit.Meteor_Hit" _returnvalue (struct) 0.6 (`KismetMathLibrary.RandomFloatInRange` 0.1 2.0) 0.0 null null null null)
      (set `self.Timer` 0.0)
      (`/Game/Dynamics/Blueprints/BP_ImpactZone.FadeOut` (`self.ImpactDecal`))
      (`self.K2_DestroyActor`))))

(event `self.ReceiveTick`
  (params (DeltaSeconds :type "Float (single-precision)"))
  (bind _impactdecal (`self.ImpactDecal`))
  ;[1 1 1] Increase timer
  (bind _output_get (set `self.Timer` (+ (`self.Timer`) (`GameplayStatics.GetWorldDeltaSeconds`))))
  (if (> _output_get 10.0)
    ;;[1 1 1] Failsafe for non-compliant meteors
    (`/Engine/EditorBlueprintResources/StandardMacros.DoOnce` false
      (:`Completed`
        (if (`KismetSystemLibrary.IsValid` _impactdecal)
          (`/Game/Dynamics/Blueprints/BP_ImpactZone.FadeOut` _impactdecal))
        (`self.K2_DestroyActor`)))))

(event `self.ReceiveBeginPlay`
  (bind _returnvalue (`self.K2_GetActorLocation`))
  ;[1 1 1] Spawn Impact Zone
  (bind (_outhit _returnvalue_2) (`KismetSystemLibrary.LineTraceSingle` _returnvalue (+ _returnvalue (* (`KismetMathLibrary.MakeVector` 0.0 0.0 -1.0) 50000.0)) "TraceTypeQuery1"))
  (if _returnvalue_2
    (bind _returnvalue_3 (`|SpawnActorFromClass` "/Game/Dynamics/Blueprints/BP_ImpactZone.BP_ImpactZone_C" (`KismetMathLibrary.MakeTransform` (`.Location` (`GameplayStatics.BreakHitResult` _outhit))) "Undefined" "MultiplyWithRoot" null null))
    (bind _output_get (set `self.ImpactDecal` _returnvalue_3))
    (`/Game/Dynamics/Blueprints/BP_ImpactZone.FadeIn` _output_get)
    (else
      (`KismetSystemLibrary.PrintString` "Couldn't spawn Impact Zone. Meteor found no floor."))))

(fn `UserConstructionScript`)