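; BP_HealthBoost is a power-up pickup that triggers when a BP_PlayerCharacter overlaps its Collider.
; A DoOnce limits it to a single activation, which calls PowerUp on the player, plays a camera shutter sound and prints PowerUpName.
; It then passes the player to ApplyEffect, whose logic is not defined in these graphs, and the actor is not destroyed here.
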(event `self.ReceiveBeginPlay`
  (`parent.ReceiveBeginPlay`))

(event `self.Collider.OnComponentBeginOverlap`
  (params (OverlappedComponent :type "PrimitiveComponent Object Reference") (OtherActor :type "Actor Object Reference") (OtherComp :type "PrimitiveComponent Object Reference") (OtherBodyIndex :type Integer) (bFromSweep :type Boolean) (SweepResult :type "HitResult Structure (by ref)"))
  (bind _asbp_player_character (cast `/Game/Dynamics/PlayerCharacter/Blueprints/BP_PlayerCharacter` OtherActor))
  (`/Engine/EditorBlueprintResources/StandardMacros.DoOnce` false
    (:`Completed`
      (`/Game/Dynamics/PlayerCharacter/Blueprints/BP_PlayerCharacter.PowerUp` _asbp_player_character null)
      (`GameplayStatics.PlaySound2D` "/Engine/VREditor/Sounds/UI/Camera_Shutter.Camera_Shutter" 1.0 1.0 0.0 null null)
      (`KismetSystemLibrary.PrintString` (`self.PowerUpName`))
      (`self.ApplyEffect` _asbp_player_character))))

(fn `UserConstructionScript`
  (`parent.UserConstructionScript`))