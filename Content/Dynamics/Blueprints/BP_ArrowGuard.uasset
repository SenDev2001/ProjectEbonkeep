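; BP_ArrowGuard is an arrow projectile that damages what it hits and sticks into it.
; It ignores its instigator and turns to face its velocity each tick until it slows down.
; The Bullet component's hit applies damage and plays a sound.
; The actor's Hit event stops movement, disables physics and collision, then attaches to the hit component and destroys the arrow after a delay.
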(event `self.ReceiveBeginPlay`
  ;[1 1 1] Don't collide with owner
  (`PrimitiveComponent.IgnoreActorWhenMoving` (`self.Bullet`) (`self.GetInstigator`) true))

(event `self.Bullet.OnComponentHit`
  (params (HitComponent :type "PrimitiveComponent Object Reference") (OtherActor :type "Actor Object Reference") (OtherComp :type "PrimitiveComponent Object Reference") (NormalImpulse :type "Vector Structure") (Hit :type "HitResult Structure (by ref)"))
  ;[1 1 1] On hit, deal damage
  (if (!= OtherActor (`self.GetInstigator`))
    (`GameplayStatics.ApplyDamage` OtherActor 20.0)
    (`GameplayStatics.PlaySoundAtLocation` "/Engine/EngineSounds/1kSineTonePing.1kSineTonePing" (`SceneComponent.RelativeLocation` (`self.Bullet`)) (struct) 1.0 1.0 0.0 null null null null)))

(event `self.ReceiveTick`
  (params (DeltaSeconds :type "Float (single-precision)"))
  (bind _velocity (`MovementComponent.Velocity` (`self.ProjectileMovement`)))
  ;[1 1 1] Calculate Rotation During Flight
  (if (not (< (`KismetMathLibrary.VSize` _velocity) 130.0))
    (`self.K2_SetActorRotation` (`KismetMathLibrary.MakeRotFromX` _velocity))))

(event `self.ReceiveHit`
  (params (MyComp :type "PrimitiveComponent Object Reference") (Other :type "Actor Object Reference") (OtherComp :type "PrimitiveComponent Object Reference") (bSelfMoved :type Boolean) (HitLocation :type "Vector Structure") (HitNormal :type "Vector Structure") (NormalImpulse :type "Vector Structure") (Hit :type "HitResult Structure (by ref)"))
  (bind (_bblockinghit _binitialoverlap _time _distance _location _impactpoint _normal _impactnormal _physmat _hitactor _hitcomponent) (`GameplayStatics.BreakHitResult` Hit))
  (bind _bullet (`self.Bullet`))
  ;[1 1 1] Attempt to stick to target
  (if (!= Other (`self.GetInstigator`))
    (set `MovementComponent.Velocity` (0.0 0.0 0.0) (`self.ProjectileMovement`))
    (`PrimitiveComponent.SetSimulatePhysics` _bullet false)
    (`PrimitiveComponent.SetCollisionEnabled` _bullet "NoCollision")
    (if (!= (`self.Bullet`) _hitcomponent)
      (`self.K2_AttachToComponent` _hitcomponent "None" "KeepWorld" "KeepWorld" "KeepWorld")
      (`KismetSystemLibrary.Delay` 5.0)
      (`self.K2_DestroyActor`))))

(fn `UserConstructionScript`)