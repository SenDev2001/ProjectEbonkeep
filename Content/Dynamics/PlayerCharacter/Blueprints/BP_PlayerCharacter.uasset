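; Player character Blueprint that handles aiming, sprinting, crouching, shooting, health and death.
; Enhanced Input events adjust walk speed and camera FOV, with aiming blocking sprint, and spawn BP_Bullet at ProjectileSpawnPos.
; Damage updates the WB_Main health UI and spawns an explosion effect.
; At zero health the mesh ragdolls, then after a delay the character moves to a PlayerStart with animation, movement and health restored.
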(event `self.ReceiveBeginPlay`
  (`parent.ReceiveBeginPlay`)
  ;[1 1 1] Add main UI & set usable WBMain variable reference
  (bind _returnvalue (`|CreateWidget` "/Game/Dynamics/Blueprints/WidgetBlueprints/WB_Main.WB_Main_C"))
  (bind _output_get (set `self.WB_Main` _returnvalue))
  (`UserWidget.AddToViewport` _output_get 0)
  ;[1 1 1] Add alt UI
  (bind _returnvalue_2 (`|CreateWidget` "/Game/Dynamics/Blueprints/WidgetBlueprints/WB_Crosshair.WB_Crosshair_C"))
  (`UserWidget.AddToViewport` _returnvalue_2 0)
  ;[0.05098 0.05098 0.05098] Add Player Input Mapping (Stolen from third person BP)
  (bind _asplayer_controller (cast `PlayerController` (`self.GetController`)))
  (bind _returnvalue_3 (pcsubsystem `EnhancedInputLocalPlayerSubsystem` _asplayer_controller))
  (`/Engine/EditorBlueprintResources/StandardMacros.IsValid` _returnvalue_3
    (:`Is Valid`
      (`EnhancedInputSubsystemInterface.AddMappingContext` _returnvalue_3 "/Game/Dynamics/PlayerCharacter/Input/PlayerInputMap.PlayerInputMap" 0 (struct))
      (`self.InitHealth`))
    (:`Is Not Valid`
      (`KismetSystemLibrary.PrintString` "Failed Input system"))))

(event `InitHealth`
  (bind _output_get (set `self.CurrentHealth` (`self.MaxHealth`)))
  (`/Game/Dynamics/Blueprints/WidgetBlueprints/WB_Main.UpdateHealthUI` (`self.WB_Main`) _output_get (`self.MaxHealth`)))

(event `EnhancedInput|/Game/Dynamics/PlayerCharacter/Input/Actions/IA_Aim`
  (params (ActionValue :type "Vector Structure") (ElapsedSeconds :type "Float (double-precision)") (TriggeredSeconds :type "Float (double-precision)") (InputAction :type "InputAction Object Reference" :default "/Game/Dynamics/PlayerCharacter/Input/Actions/IA_Aim.IA_Aim"))
  (bind _followcamera (`self.FollowCamera`))
  (bind _charactermovement (`self.CharacterMovement`))
  ;[1 1 1] Aim
  (:`Triggered`
    (set `self.IsAiming?` true :!label _label)
    (set `CharacterMovementComponent.MaxWalkSpeed` 170.0 _charactermovement)
    (`CameraComponent.SetFieldOfView` _followcamera 70.0))
  (:`Ongoing`
    (goto _label))
  (:`Completed`
    (set `self.IsAiming?` false)
    (set `CharacterMovementComponent.MaxWalkSpeed` 300.0 _charactermovement)
    (`CameraComponent.SetFieldOfView` _followcamera 90.0)))

(event `self.ReceiveAnyDamage`
  (params (Damage :type "Float (single-precision)") (DamageType :type "DamageType Object Reference") (InstigatedBy :type "Controller Object Reference") (DamageCauser :type "Actor Object Reference"))
  (if (not (`self.bIsDead`))
    (bind _output_get (set `self.CurrentHealth` (`KismetMathLibrary.FClamp` (- (`self.CurrentHealth`) Damage) 0.0 (`self.MaxHealth`))))
    (`/Game/Dynamics/Blueprints/WidgetBlueprints/WB_Main.UpdateHealthUI` (`self.WB_Main`) _output_get (`self.MaxHealth`))
    (`GameplayStatics.SpawnEmitterAtLocation` "/Game/StarterContent/Particles/P_Explosion.P_Explosion" (`self.K2_GetActorLocation`))
    (if (== (`self.CurrentHealth`) 0.0)
      (`self.OnDeath`))))

(event `EnhancedInput|/Game/Dynamics/PlayerCharacter/Input/Actions/IA_Sprint`
  (params (ActionValue :type Boolean) (ElapsedSeconds :type "Float (double-precision)") (TriggeredSeconds :type "Float (double-precision)") (InputAction :type "InputAction Object Reference" :default "/Game/Dynamics/PlayerCharacter/Input/Actions/IA_Sprint.IA_Sprint"))
  (bind _charactermovement (`self.CharacterMovement`))
  ;[1 1 1] Sprint
  (:`Triggered`
    (if (not (`self.IsAiming?`)) :!label _label_2
      (set `CharacterMovementComponent.MaxWalkSpeed` 600.0 _charactermovement)))
  (:`Started`
    (goto _label_2))
  (:`Ongoing`
    (goto _label_2))
  (:`Canceled`
    (set `CharacterMovementComponent.MaxWalkSpeed` 300.0 _charactermovement :!label _label_3))
  (:`Completed`
    (goto _label_3)))

(event `OnDeath`
  (bind _mesh (`self.Mesh`))
  (bind _charactermovement (`self.CharacterMovement`))
  (set `self.bIsDead` true)
  (`PrimitiveComponent.SetSimulatePhysics` _mesh true)
  (`PrimitiveComponent.AddForce` _mesh (0.0 0.0 1000.0) "None" false)
  (`CharacterMovementComponent.DisableMovement` _charactermovement)
  (`MovementComponent.StopMovementImmediately` _charactermovement)
  (`KismetSystemLibrary.Delay` 3.0)
  (`self.Respawn`))

(event `EnhancedInput|/Game/Dynamics/PlayerCharacter/Input/Actions/IA_PlayerShoot`
  (params (ActionValue :type Boolean) (ElapsedSeconds :type "Float (double-precision)") (TriggeredSeconds :type "Float (double-precision)") (InputAction :type "InputAction Object Reference" :default "/Game/Dynamics/PlayerCharacter/Input/Actions/IA_PlayerShoot.IA_PlayerShoot"))
  (bind (_returnvalue_location _returnvalue_rotation) (`KismetMathLibrary.BreakTransform` (`SceneComponent.K2_GetComponentToWorld` (`self.Projectile Spawn Pos`))))
  ;[1 1 1] Shoot projectile
  (:`Started`
    (`|SpawnActorFromClass` "/Game/Dynamics/Blueprints/BP_Bullet.BP_Bullet_C" (`KismetMathLibrary.MakeTransform` _returnvalue_location _returnvalue_rotation (0.2 0.2 0.2)) "AlwaysSpawn" "MultiplyWithRoot" null null)))

(event `Respawn`
  (bind _mesh (`self.Mesh`))
  (set `self.bIsDead` false)
  (bind _returnvalue (`GameplayStatics.GetActorOfClass` "/Script/Engine.PlayerStart"))
  (`self.K2_SetActorLocation` (`self.K2_GetActorLocation` _returnvalue))
  (`CharacterMovementComponent.SetMovementMode` (`self.CharacterMovement`) "MOVE_Walking" 0)
  (`SkeletalMeshComponent.SetAnimInstanceClass` _mesh "/Game/Statics/Characters/Mannequins/Animations/ABP_Quinn.ABP_Quinn_C")
  (`PrimitiveComponent.SetSimulatePhysics` _mesh false)
  (`self.InitHealth`))

(event `EnhancedInput|/Game/Dynamics/PlayerCharacter/Input/Actions/IA_Crouch`
  (params (ActionValue :type Boolean) (ElapsedSeconds :type "Float (double-precision)") (TriggeredSeconds :type "Float (double-precision)") (InputAction :type "InputAction Object Reference" :default "/Game/Dynamics/PlayerCharacter/Input/Actions/IA_Crouch.IA_Crouch"))
  ;[1 1 1] Crouch
  (:`Triggered`
    (`self.Crouch`))
  (:`Completed`
    (`self.UnCrouch`)))

(fn `UserConstructionScript`
  (`parent.UserConstructionScript`))