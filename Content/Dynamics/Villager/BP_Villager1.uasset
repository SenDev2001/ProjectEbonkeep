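; Villager NPC that wanders the level and reacts when the player comes close.
; A self-restarting AIMoveTo loop picks random reachable points around its current location, repeating only on success.
; The PlayerDetection overlap flags the player as near and zeroes movement without explicitly aborting the move, then calls the wander again on exit.
; AI perception stores the seen state and player reference, which nothing here uses to steer behavior.
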(event `self.ReceiveBeginPlay`
  (`self.NPC MOve`))

(event `NPC MOve`
  (`|AIMoveTo` self (`NavigationSystemV1.K2_GetRandomReachablePointInRadius` (`self.K2_GetActorLocation`) 2500.0 null null) null 100.0
    (:`OnSuccess`
      (`self.NPC MOve`))))

(event `self.AIPerception.OnTargetPerceptionUpdated`
  (params (Actor :type "Actor Object Reference") (Stimulus :type "AIStimulus Structure"))
  (bind _output_get (set `self.Seen_Player` Stimulus_bSuccessfullySensed))
  (if _output_get
    (bind _asbp_player_character (cast `/Game/Dynamics/PlayerCharacter/Blueprints/BP_PlayerCharacter` Actor))
    (set `self.Player reference` _asbp_player_character)))

(event `self.Player Detection.OnComponentBeginOverlap`
  (params (OverlappedComponent :type "PrimitiveComponent Object Reference") (OtherActor :type "Actor Object Reference") (OtherComp :type "PrimitiveComponent Object Reference") (OtherBodyIndex :type Integer) (bFromSweep :type Boolean) (SweepResult :type "HitResult Structure (by ref)"))
  (cast `/Game/Dynamics/PlayerCharacter/Blueprints/BP_PlayerCharacter` OtherActor)
  (set `self.IsPlayerNear` true)
  (`MovementComponent.StopMovementImmediately` (`self.CharacterMovement`)))

(event `self.Player Detection.OnComponentEndOverlap`
  (params (OverlappedComponent :type "PrimitiveComponent Object Reference") (OtherActor :type "Actor Object Reference") (OtherComp :type "PrimitiveComponent Object Reference") (OtherBodyIndex :type Integer))
  (cast `/Game/Dynamics/PlayerCharacter/Blueprints/BP_PlayerCharacter` OtherActor)
  (set `self.IsPlayerNear` false)
  (`self.NPC MOve`))

(fn `UserConstructionScript`)