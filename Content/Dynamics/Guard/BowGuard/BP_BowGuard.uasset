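; Bow-wielding enemy guard with health, a camera-facing health bar, and ranged attacks on its AI focus actor.
; Tick updates the bar and calls FireArrow, which traces from HitPoint, spawns BP_Arrow after a two-second delay, then plays effects if the trace hit the player.
; Damage lowers health; exactly zero triggers ragdoll and delayed destruction.
; Helper functions expose the patrol route and set walk speed by movement state.
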(event `InitHealth`
  ;[0 1 0.1887] InitHealth
  (bind _output_get (set `self.CurrentHealth` (`self.MaxHealth`)))
  (`ProgressBar.SetPercent` (`/Game/Dynamics/Guard/WB_EnemyHealthBar.HealthBarEnemy` (`self.GuardHealth`)) (/ _output_get (`self.MaxHealth`))))

(event `self.ReceiveBeginPlay`
  ;[0 0.5753 1] Begin Play Setup
  (`parent.ReceiveBeginPlay`)
  (bind _returnvalue (`|CreateWidget` "/Game/Dynamics/Guard/WB_EnemyHealthBar.WB_EnemyHealthBar_C"))
  (set `self.GuardHealth` _returnvalue)
  (`self.InitHealth`))

(event `self.ReceiveAnyDamage`
  (params (Damage :type "Float (single-precision)") (DamageType :type "DamageType Object Reference") (InstigatedBy :type "Controller Object Reference") (DamageCauser :type "Actor Object Reference"))
  ;[1 0.3284 0] On take damage, check if dead, remove hp, trigger death if dead
  (set `self.CurrentHealth` (- (`self.CurrentHealth`) Damage))
  (if (== (`self.CurrentHealth`) 0.0)
    (`self.On Death`)))

(event `self.ReceiveTick`
  (params (DeltaSeconds :type "Float (single-precision)"))
  (bind _healthbarwidget (`self.HealthBarWidget`))
  ;[1 0.2722 0.8293] Event Tick
  (`|ExecutionSequence`
    (:`then_0`
      (bind _aswb_enemy_health_bar (cast `/Game/Dynamics/Guard/WB_EnemyHealthBar` (`WidgetComponent.GetWidget` (`self.HealthBarWidget`))))
      (`ProgressBar.SetPercent` (`/Game/Dynamics/Guard/WB_EnemyHealthBar.HealthBarEnemy` _aswb_enemy_health_bar) (/ (`self.CurrentHealth`) (`self.MaxHealth`)))
      (`SceneComponent.K2_SetWorldRotation` _healthbarwidget (`KismetMathLibrary.FindLookAtRotation` (`SceneComponent.K2_GetComponentLocation` _healthbarwidget) (`SceneComponent.K2_GetComponentLocation` (`PlayerCameraManager.TransformComponent` (`GameplayStatics.GetPlayerCameraManager` 0)))) false false))
    (:`then_1`
      (`self.FireArrow`))))

(event `On Death`
  ;[1 0 0] OnDeath
  (set `self.IsDead?` true)
  (`CharacterMovementComponent.DisableMovement` (`self.CharacterMovement`))
  (`PrimitiveComponent.SetSimulatePhysics` (`self.Mesh`) true)
  (`KismetSystemLibrary.Delay` 3.0)
  (`self.K2_DestroyActor`))

(event `FireArrow`
  (bind (_returnvalue_location _returnvalue_rotation _returnvalue_scale) (`KismetMathLibrary.BreakTransform` (`SceneComponent.K2_GetComponentToWorld` (`self.Hit point`))))
  (bind _returnvalue (`AIController.GetFocusActor` (`AIBlueprintHelperLibrary.GetAIController` self)))
  ;[1 0.433 0.3832] Attack Stuff
  (`/Engine/EditorBlueprintResources/StandardMacros.IsValid` _returnvalue
    (:`Is Valid`
      (bind _outhit (`KismetSystemLibrary.LineTraceSingle` (`SceneComponent.K2_GetComponentLocation` (`self.Hit point`)) (`self.K2_GetActorLocation` _returnvalue) "TraceTypeQuery1"))
      (`KismetSystemLibrary.Delay` 2.0)
      (bind (_bblockinghit _binitialoverlap _time _distance _location _impactpoint _normal _impactnormal _physmat _hitactor _hitcomponent _hitbonename _bonename _hititem _elementindex _faceindex _tracestart _traceend) (`GameplayStatics.BreakHitResult` _outhit))
      (bind _returnvalue_2 (`KismetMathLibrary.FindLookAtRotation` _tracestart _traceend))
      (`|SpawnActorFromClass` "/Game/Dynamics/Blueprints/BP_Arrow.BP_Arrow_C" (`KismetMathLibrary.MakeTransform` _returnvalue_location _returnvalue_2 _returnvalue_scale) "AlwaysSpawn" "OverrideRootScale" (`self.GetOwner`) self)
      (if true
        (bind _asbp_player_character (cast `/Game/Dynamics/PlayerCharacter/Blueprints/BP_PlayerCharacter` _hitactor))
        (`GameplayStatics.PlaySound2D` "/Game/Dynamics/Guard/BowGuard/videoplayback_01.videoplayback_01" 2.0 1.0 0.0 null _asbp_player_character)
        (`NiagaraFunctionLibrary.SpawnSystemAtLocation` null (0.0 0.0 0.0) _returnvalue_2)))))

(fn `GetPatrolRoute`
  (returns (PatrolRoute :type "/Game/Dynamics/Guard/SwordGuard/AI/BP_PatrolRoute Object Reference"))
  (return (`self.PatrolRoute`)))

(fn `Patrolroute 1`
  (returns (PatrolRoute :type "/Game/Dynamics/Guard/SwordGuard/AI/BP_PatrolRoute Object Reference"))
  (return (`self.PatrolRoute`)))

(fn `SetMovementSpeed`
  (params (Speed :type "/Game/Dynamics/Guard/SwordGuard/AI/ENUM/E_MovementSpeed Enum" :default "NewEnumerator0"))
  (returns (SpeedValue :type "Float (double-precision)"))
  (bind _output_get (set `CharacterMovementComponent.MaxWalkSpeed` (select `/Game/Dynamics/Guard/SwordGuard/AI/ENUM/E_MovementSpeed` Speed :`NewEnumerator1` 100.0 :`NewEnumerator2` 300.0 :`NewEnumerator3` 500.0 :!type "Float (single-precision)") (`self.CharacterMovement`)))
  (return _output_get))

(fn `UserConstructionScript`)