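; BP_Shockwave is an expanding shockwave actor that damages the player once and pairs with a Niagara effect.
; On BeginPlay a timeline scales a collision sphere outward over time.
; The first overlap with the player character applies fixed damage through a DoOnce gate.
; The actor destroys itself when the Niagara system finishes.
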(event `self.ReceiveBeginPlay`
  (bind (_direction _shockwave) (`Timeline|ShockwaveTimeline`)
    (:`Update`
      (`SceneComponent.SetWorldScale3D` (`self.Sphere`) (`KismetMathLibrary.Conv_DoubleToVector` _shockwave)))))

(event `self.Sphere.OnComponentBeginOverlap`
  (params (OverlappedComponent :type "PrimitiveComponent Object Reference") (OtherActor :type "Actor Object Reference") (OtherComp :type "PrimitiveComponent Object Reference") (OtherBodyIndex :type Integer) (bFromSweep :type Boolean) (SweepResult :type "HitResult Structure (by ref)"))
  (if (== OtherActor (`GameplayStatics.GetPlayerCharacter` 0))
    (`/Engine/EditorBlueprintResources/StandardMacros.DoOnce` false
      (:`Completed`
        (`GameplayStatics.ApplyDamage` OtherActor 30.0)))))

(event `self.NS_ShockwaveAttemptTwo_FX.OnSystemFinished`
  (params (PSystem :type "NiagaraComponent Object Reference"))
  (`self.K2_DestroyActor`))

(fn `UserConstructionScript`)