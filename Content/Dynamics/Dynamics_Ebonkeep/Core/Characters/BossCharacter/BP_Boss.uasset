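; Boss character for Ebonkeep, built on a CastleGuard01 mesh, with a simple health pool and two ways to be taken out.
; Damage lowers clamped health and spawns a large explosion; at zero, OnDeath flags it dead and switches the mesh to physics ragdoll.
; Separately, any overlap on the body, head or either arm collider bypasses health, playing an explosion with world-origin sound and destroying the actor immediately.
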(event `InitHealth`
  (set `self.CurrentHealth` (`self.MaxHealth`)))

(event `self.ReceiveBeginPlay`
  (`self.InitHealth`))

(event `self.ReceiveAnyDamage`
  (params (Damage :type "Float (single-precision)") (DamageType :type "DamageType Object Reference") (InstigatedBy :type "Controller Object Reference") (DamageCauser :type "Actor Object Reference"))
  ;[1 1 1] On take damage, check if dead, remove hp, update health UI, trigger death if dead
  (if (not (`self.IsDead`))
    (set `self.CurrentHealth` (`KismetMathLibrary.FClamp` (- (`self.CurrentHealth`) Damage) 0.0 (`self.MaxHealth`)))
    (`GameplayStatics.SpawnEmitterAtLocation` "/Game/Statics/StarterContent/Particles/P_Explosion.P_Explosion" (`SkeletalMeshComponent.GetSkeletalCenterOfMass` (`self.castle_guard_01`)) (struct) (10.0 10.0 10.0))
    (if (== (`self.CurrentHealth`) 0.0)
      (`self.OnDeath`))))

(event `self.BodyCollider.OnComponentBeginOverlap`
  (params (OverlappedComponent :type "PrimitiveComponent Object Reference") (OtherActor :type "Actor Object Reference") (OtherComp :type "PrimitiveComponent Object Reference") (OtherBodyIndex :type Integer) (bFromSweep :type Boolean) (SweepResult :type "HitResult Structure (by ref)"))
  (`GameplayStatics.SpawnEmitterAtLocation` "/Game/Statics/StarterContent/Particles/P_Explosion.P_Explosion" (`SkeletalMeshComponent.GetSkeletalCenterOfMass` (`self.castle_guard_01`)) (struct) (3.0 3.0 3.0) :!label _label)
  (`GameplayStatics.PlaySoundAtLocation` "/Game/Statics/StarterContent/Audio/Explosion01.Explosion01" (0.0 0.0 0.0) (struct) 1.0 1.0 0.0 null null null null)
  (`self.K2_DestroyActor`))

(event `self.ArmCollider.OnComponentBeginOverlap`
  (params (OverlappedComponent :type "PrimitiveComponent Object Reference") (OtherActor :type "Actor Object Reference") (OtherComp :type "PrimitiveComponent Object Reference") (OtherBodyIndex :type Integer) (bFromSweep :type Boolean) (SweepResult :type "HitResult Structure (by ref)"))
  (goto _label))

(event `self.Head.OnComponentBeginOverlap`
  (params (OverlappedComponent :type "PrimitiveComponent Object Reference") (OtherActor :type "Actor Object Reference") (OtherComp :type "PrimitiveComponent Object Reference") (OtherBodyIndex :type Integer) (bFromSweep :type Boolean) (SweepResult :type "HitResult Structure (by ref)"))
  (goto _label))

(event `self.ArmCollider2.OnComponentBeginOverlap`
  (params (OverlappedComponent :type "PrimitiveComponent Object Reference") (OtherActor :type "Actor Object Reference") (OtherComp :type "PrimitiveComponent Object Reference") (OtherBodyIndex :type Integer) (bFromSweep :type Boolean) (SweepResult :type "HitResult Structure (by ref)"))
  (goto _label))

(fn `OnDeath`
  (bind _castle_guard_01 (`self.castle_guard_01`))
  (set `self.IsDead` true)
  (`PrimitiveComponent.SetSimulatePhysics` _castle_guard_01 true)
  (`SkeletalMeshComponent.SetPhysicsBlendWeight` _castle_guard_01 1.0)
  (`PrimitiveComponent.SetCollisionEnabled` _castle_guard_01 "QueryAndPhysics"))

(fn `UserConstructionScript`)