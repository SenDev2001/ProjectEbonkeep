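; Third-person player character with health, sprint, crouch, aim, shooting and ragdoll death followed by respawn at a PlayerStart.
; BeginPlay creates the HUD, crosshair and input mapping, and damage updates health UI.
; Held fire repeats hitscan shots: a screen-center camera trace sets the target for a muzzle trace that applies damage and triggers a FS_MasterField at impact.
; Debug keys emit noise and report damage events for testing guard AI senses.
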(event `self.ReceiveBeginPlay`
  (`parent.ReceiveBeginPlay`)
  ;[1 1 1] Add main UI & set usable WBMain variable reference
  (bind _returnvalue (`|CreateWidget` "/Game/Dynamics/Dynamics_Ebonkeep/Other_Blueprints/WidgetBlueprints/WB_Main.WB_Main_C"))
  (bind _output_get (set `self.WB_Main` _returnvalue))
  (`UserWidget.AddToViewport` _output_get 0)
  ;[1 1 1] Add alt UI
  (bind _returnvalue_2 (`|CreateWidget` "/Game/Dynamics/Dynamics_Ebonkeep/Other_Blueprints/WidgetBlueprints/WB_Crosshair.WB_Crosshair_C"))
  (`UserWidget.AddToViewport` _returnvalue_2 0)
  ;[0.05098 0.05098 0.05098] Add Player Input Mapping (Stolen from third person BP)
  (bind _asplayer_controller (cast `PlayerController` (`self.GetController`)))
  (bind _returnvalue_3 (pcsubsystem `EnhancedInputLocalPlayerSubsystem` _asplayer_controller))
  (`/Engine/EditorBlueprintResources/StandardMacros.IsValid` _returnvalue_3
    (:`Is Valid`
      (`EnhancedInputSubsystemInterface.AddMappingContext` _returnvalue_3 "/Game/Dynamics/Dynamics_Ebonkeep/Core/Characters/PlayerCharacter/Input/PlayerInputMap.PlayerInputMap" 0 (struct))
      (`self.InitHealth`))
    (:`Is Not Valid`
      (`KismetSystemLibrary.PrintString` "Failed Input system"))))

(event `InitHealth`
  (bind _output_get (set `self.CurrentHealth` (`self.MaxHealth`)))
  (`/Game/Dynamics/Dynamics_Ebonkeep/Other_Blueprints/WidgetBlueprints/WB_Main.UpdateHealthUI` (`self.WB_Main`) _output_get (`self.MaxHealth`)))

(event `self.ReceiveAnyDamage`
  (params (Damage :type "Float (single-precision)") (DamageType :type "DamageType Object Reference") (InstigatedBy :type "Controller Object Reference") (DamageCauser :type "Actor Object Reference"))
  ;[1 1 1] On take damage, check if dead, remove hp, update health UI, trigger death if dead
  (if (not (`self.bIsDead`))
    (bind _output_get (set `self.CurrentHealth` (`KismetMathLibrary.FClamp` (- (`self.CurrentHealth`) Damage) 0.0 (`self.MaxHealth`))))
    (`/Game/Dynamics/Dynamics_Ebonkeep/Other_Blueprints/WidgetBlueprints/WB_Main.UpdateHealthUI` (`self.WB_Main`) _output_get (`self.MaxHealth`))
    (`GameplayStatics.SpawnEmitterAtLocation` "/Game/Statics/StarterContent/Particles/P_Explosion.P_Explosion" (`self.K2_GetActorLocation`))
    (if (== (`self.CurrentHealth`) 0.0)
      (`self.OnDeath`))))

(event `EnhancedInput|/Game/Dynamics/Dynamics_Ebonkeep/Core/Characters/PlayerCharacter/Input/Actions/IA_Sprint`
  (params (ActionValue :type Boolean) (ElapsedSeconds :type "Float (double-precision)") (TriggeredSeconds :type "Float (double-precision)") (InputAction :type "InputAction Object Reference" :default "/Game/Dynamics/Dynamics_Ebonkeep/Core/Characters/PlayerCharacter/Input/Actions/IA_Sprint.IA_Sprint"))
  (bind _charactermovement (`self.CharacterMovement`))
  ;[1 1 1] Sprint
  (:`Triggered`
    (if (not (`self.IsAiming?`)) :!label _label
      (set `CharacterMovementComponent.MaxWalkSpeed` 500.0 _charactermovement)))
  (:`Started`
    (goto _label))
  (:`Ongoing`
    (goto _label))
  (:`Canceled`
    (set `CharacterMovementComponent.MaxWalkSpeed` 300.0 _charactermovement :!label _label_2))
  (:`Completed`
    (goto _label_2)))

(event `OnDeath`
  (bind _mesh (`self.Mesh`))
  (bind _charactermovement (`self.CharacterMovement`))
  ;[1 1 1] On death
  (set `self.bIsDead` true)
  (`PrimitiveComponent.SetSimulatePhysics` _mesh true)
  (`PrimitiveComponent.AddForce` _mesh (0.0 0.0 1000.0) "None" false)
  (`CharacterMovementComponent.DisableMovement` _charactermovement)
  (`MovementComponent.StopMovementImmediately` _charactermovement)
  (`KismetSystemLibrary.Delay` 3.0)
  (`self.Respawn`))

(event `Respawn`
  (bind _mesh (`self.Mesh`))
  ;[1 1 1] Respawn
  (set `self.bIsDead` false)
  (bind _returnvalue (`GameplayStatics.GetActorOfClass` "/Script/Engine.PlayerStart"))
  (`self.K2_SetActorLocation` (`self.K2_GetActorLocation` _returnvalue))
  (`CharacterMovementComponent.SetMovementMode` (`self.CharacterMovement`) "MOVE_Walking" 0)
  (`SkeletalMeshComponent.SetAnimInstanceClass` _mesh "/Game/Statics/Characters/Mannequins/Animations/ABP_Quinn.ABP_Quinn_C")
  (`PrimitiveComponent.SetSimulatePhysics` _mesh false)
  (`self.InitHealth`))

(event `EnhancedInput|/Game/Dynamics/Dynamics_Ebonkeep/Core/Characters/PlayerCharacter/Input/Actions/IA_Crouch`
  (params (ActionValue :type Boolean) (ElapsedSeconds :type "Float (double-precision)") (TriggeredSeconds :type "Float (double-precision)") (InputAction :type "InputAction Object Reference" :default "/Game/Dynamics/Dynamics_Ebonkeep/Core/Characters/PlayerCharacter/Input/Actions/IA_Crouch.IA_Crouch"))
  (bind _charactermovement (`self.CharacterMovement`))
  ;[1 1 1] Crouch
  (:`Triggered`
    (set `self.IsCrouching?` true)
    (set `CharacterMovementComponent.MaxWalkSpeed` 150.0 _charactermovement)
    (bind (_direction _newtrack_0) (`Timeline|CrouchTimeline` :!label _label_3)
      (:`Update`
        (`SceneComponent.K2_SetRelativeLocation` (`self.CameraBoom`) (`KismetMathLibrary.MakeVector` 0.0 0.0 _newtrack_0) false false))))
  (:`Completed`
    (set `self.IsCrouching?` false)
    (set `CharacterMovementComponent.MaxWalkSpeed` 500.0 _charactermovement)
    (goto _label_3 :!via `Reverse`)))

(event `EnhancedInput|/Game/Dynamics/Dynamics_Ebonkeep/Core/Characters/PlayerCharacter/Input/Actions/IA_Aim`
  (params (ActionValue :type "Vector Structure") (ElapsedSeconds :type "Float (double-precision)") (TriggeredSeconds :type "Float (double-precision)") (InputAction :type "InputAction Object Reference" :default "/Game/Dynamics/Dynamics_Ebonkeep/Core/Characters/PlayerCharacter/Input/Actions/IA_Aim.IA_Aim"))
  (bind _followcamera (`self.FollowCamera`))
  (bind _charactermovement (`self.CharacterMovement`))
  ;[1 1 1] Aim
  (:`Triggered`
    (set `self.IsAiming?` true :!label _label_4)
    (set `CharacterMovementComponent.MaxWalkSpeed` 150.0 _charactermovement)
    (`CameraComponent.SetFieldOfView` _followcamera 70.0))
  (:`Ongoing`
    (goto _label_4))
  (:`Completed`
    (set `self.IsAiming?` false)
    (set `CharacterMovementComponent.MaxWalkSpeed` 500.0 _charactermovement)
    (`CameraComponent.SetFieldOfView` _followcamera 90.0)))

(event `Key|R`
  (params (Key :type "Key Structure"))
  ;[1 1 1] Passive and Patroling switch test
)

(event `EnhancedInput|/Game/Dynamics/Dynamics_Ebonkeep/Core/Characters/PlayerCharacter/Input/Actions/IA_PlayerShoot`
  (params (ActionValue :type Boolean) (ElapsedSeconds :type "Float (double-precision)") (TriggeredSeconds :type "Float (double-precision)") (InputAction :type "InputAction Object Reference" :default "/Game/Dynamics/Dynamics_Ebonkeep/Core/Characters/PlayerCharacter/Input/Actions/IA_PlayerShoot.IA_PlayerShoot"))
  ;[1 1 1] Shoot projectile
  (:`Started`
    (set `self.IsFiring?` true)
    (if (`self.IsFiring?`) :!label _label_5
      (`self.Fire`)
      (`KismetSystemLibrary.Delay` 2.0)
      (goto _label_5)))
  (:`Completed`
    (set `self.IsFiring?` false)))

(event `Key|F`
  (params (Key :type "Key Structure"))
  (bind _returnvalue (`self.K2_GetActorLocation`))
  ;[1 1 1] Sound Detection Test
  (:`Pressed`
    (`self.MakeNoise` 1.0 self _returnvalue)
    (`GameplayStatics.SpawnEmitterAtLocation` "/Game/Statics/StarterContent/Particles/P_Explosion.P_Explosion" _returnvalue)
    (`GameplayStatics.PlaySoundAtLocation` "/Game/Statics/StarterContent/Audio/Collapse_Cue.Collapse_Cue" _returnvalue (struct) 1.0 1.0 0.0 null null null null)))

(event `Key|X`
  (params (Key :type "Key Structure"))
  ;[1 1 1] Sound Detection Test
  (:`Pressed`
    (bind _returnvalue (`GameplayStatics.GetActorOfClass` "/Game/Dynamics/Dynamics_Ebonkeep/Core/Characters/Guard/BP_Guard.BP_Guard_C"))
    (`AISense_Damage.ReportDamageEvent` _returnvalue self 10.0 (`self.K2_GetActorLocation`))))

(fn `Fire`
  (bind _returnvalue (`GameplayStatics.GetPlayerController` 0))
  (bind (_sizex _sizey) (`PlayerController.GetViewportSize` _returnvalue))
  (bind _returnvalue_2 (`PlayerCameraManager.GetCameraLocation` (`GameplayStatics.GetPlayerCameraManager` 0)))
  (bind _returnvalue_3 (`SceneComponent.K2_GetComponentLocation` (`self.ProjectileSpawnPos`)))
  (`GameplayStatics.PlaySound2D` null 1.0 1.0 0.0 null null)
  (bind _outhit (`KismetSystemLibrary.LineTraceSingle` :`Start` _returnvalue_2 :`End` (+ _returnvalue_2 (* (`.WorldDirection` (`GameplayStatics.DeprojectScreenToWorld` _returnvalue (`KismetMathLibrary.MakeVector2D` (`KismetMathLibrary.Conv_IntToDouble` (/ _sizex 2)) (`KismetMathLibrary.Conv_IntToDouble` (/ _sizey 2))))) 15000.0)) :`TraceChannel` "TraceTypeQuery3" :`DrawDebugType` "Persistent"))
  (bind (_bblockinghit _binitialoverlap _time _distance _location _impactpoint) (`GameplayStatics.BreakHitResult` _outhit))
  (if _bblockinghit
    (bind (_outhit_2 _returnvalue_4) (`KismetSystemLibrary.LineTraceSingle` :`Start` _returnvalue_3 :`End` (* (- _impactpoint _returnvalue_3) 15000.0) :`TraceChannel` "TraceTypeQuery3" :`DrawDebugType` "ForDuration"))
    (if _returnvalue_4
      (bind (_bblockinghit_2 _binitialoverlap_2 _time_2 _distance_2 _location_2 _impactpoint_2 _normal _impactnormal _physmat _hitactor) (`GameplayStatics.BreakHitResult` _outhit_2))
      (`GameplayStatics.ApplyDamage` _hitactor (`self.WeaponDamage`))
      (bind _returnvalue_5 (`|SpawnActorFromClass` "/Engine/EditorResources/FieldNodes/FS_MasterField.FS_MasterField_C" (`KismetMathLibrary.Conv_VectorToTransform` _impactpoint_2) "Undefined" "MultiplyWithRoot" null null))
      (`/Engine/EditorResources/FieldNodes/FS_MasterField.CE_Trigger` _returnvalue_5)
      (`self.K2_DestroyActor` _returnvalue_5))))

(fn `UserConstructionScript`
  (`parent.UserConstructionScript`))