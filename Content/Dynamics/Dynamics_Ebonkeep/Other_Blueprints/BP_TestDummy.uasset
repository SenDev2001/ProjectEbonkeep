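; BP_TestDummy is a damageable test actor that tracks its own health and is destroyed when it runs out.
; Health starts at the maximum on BeginPlay, and AnyDamage subtracts incoming damage, clamped between zero and max, while spawning an explosion effect at the actor's location.
; Reaching zero calls OnDeath, which sets the dead flag that blocks further damage and destroys the actor.
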(event `InitHealth`
  (set `self.CurrentHealth` (`self.MaxHealth`)))

(event `self.ReceiveBeginPlay`
  (`parent.ReceiveBeginPlay`)
  (`self.InitHealth`))

(event `self.ReceiveAnyDamage`
  (params (Damage :type "Float (single-precision)") (DamageType :type "DamageType Object Reference") (InstigatedBy :type "Controller Object Reference") (DamageCauser :type "Actor Object Reference"))
  ;[1 1 1] On take damage, check if dead, remove hp, update health UI, trigger death if dead
  (if (not (`self.IsDead`))
    (set `self.CurrentHealth` (`KismetMathLibrary.FClamp` (- (`self.CurrentHealth`) Damage) 0.0 (`self.MaxHealth`)))
    (`GameplayStatics.SpawnEmitterAtLocation` "/Game/Statics/StarterContent/Particles/P_Explosion.P_Explosion" (`self.K2_GetActorLocation`))
    (if (== (`self.CurrentHealth`) 0.0)
      (`self.OnDeath`))))

(fn `OnDeath`
  (set `self.IsDead` true)
  (`self.K2_DestroyActor`))

(fn `UserConstructionScript`
  (`parent.UserConstructionScript`))