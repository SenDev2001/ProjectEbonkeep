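; BP_Boss is the boss fight character, with health, a melee attack and death handling, linked to BP_AI_Boss.
; Damage updates a WB_BossFightHealth widget and the blackboard health percentage, and zero health enables ragdoll and sets bIsDead.
; Attack plays a slash montage whose notify sphere-traces for the player, applies damage and shakes the camera.
; A one-shot overlap sphere flags the target as seen and starts a looping timer that turns the boss toward the player.
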(event `self.ReceiveBeginPlay`
  ;[0 0.3914 1] Begin Play
  (bind _returnvalue (`|CreateWidget` "/Game/Dynamics/Blueprints/WidgetBlueprints/WB_BossFightHealth.WB_BossFightHealth_C"))
  (`UserWidget.AddToViewport` _returnvalue 0)
  (set `self.BossHealth` _returnvalue)
  (`self.InitHealth`)
  (`self.UpdateBossHealthBar`)
  (`KismetSystemLibrary.Delay` 0.01) ; Necessary delay for BP_AI to intialize.\nOtherwise, it does not cast properly.
  (`self.UpdateBlackboardHP`)
  (bind _asbp_player_character (cast `/Game/Dynamics/PlayerCharacter/Blueprints/BP_PlayerCharacter` (`GameplayStatics.GetPlayerCharacter` 0)))
  (set `self.PlayerCharRef` _asbp_player_character))

(event `OnDeath`
  ;[1 0.02706 0.03303] Death
  (`CharacterMovementComponent.DisableMovement` (`self.CharacterMovement`))
  (`PrimitiveComponent.SetSimulatePhysics` (`self.Mesh`) true)
  (bind _asbp_ai_boss (cast `/Game/Dynamics/BossFight/BP_AI_Boss` (`self.GetController`)))
  (`BlackboardComponent.SetValueAsBool` (`AIBlueprintHelperLibrary.GetBlackboard` _asbp_ai_boss) (`KismetStringLibrary.Conv_StringToName` "bIsDead") true)
  (set `self.isDead?` true))

(event `self.ReceiveAnyDamage`
  (params (Damage :type "Float (single-precision)") (DamageType :type "DamageType Object Reference") (InstigatedBy :type "Controller Object Reference") (DamageCauser :type "Actor Object Reference"))
  ;[1 0.5511 0] Take Damage
  (set `self.CurrentHealth` (- (`self.CurrentHealth`) Damage))
  (`self.UpdateBossHealthBar`)
  (`self.UpdateBlackboardHP`)
  (if (<= (`self.CurrentHealth`) 0.0)
    (`self.OnDeath`)))

(event `InitHealth`
  ;[0.3523 1 0] Init health
  (set `self.CurrentHealth` (`self.MaxHealth`))
  (`self.UpdateBossHealthBar`)
  (`self.UpdateBlackboardHP`))

(event `/Game/Dynamics/BossFight/BPI_BossFight.Attack`
  (bind _attack_pos (`self.Attack Pos`))
  (bind _returnvalue (`SceneComponent.K2_GetComponentLocation` _attack_pos))
  ;[0.3355 0.8412 1] Attack
  (if (and (not (`self.isAttacking?`)) (not (`self.isDead?`)))
    (`|PlayMontage` (`self.Mesh`) "/Game/Dynamics/BossFight/Animations/Sword_And_Shield_Slash_Montage.Sword_And_Shield_Slash_Montage"
      (:`then`
        (set `self.isAttacking?` true))
      (:`OnCompleted`
        (set `self.isAttacking?` false))
      (:`OnNotifyBegin`
        (`|ExecutionSequence`
          (:`then_0`
            (bind (_outhit _returnvalue_2) (`KismetSystemLibrary.SphereTraceSingleForObjects` :`Start` _returnvalue :`End` (+ _returnvalue (* (`KismetMathLibrary.GetForwardVector` (`SceneComponent.K2_GetComponentRotation` _attack_pos)) 2000.0)) :`Radius` 800.0 :`ObjectTypes` (`|MakeArray` "ObjectTypeQuery3" :!type "EObjectTypeQuery Enum") :`DrawDebugType` "ForDuration" :`DrawTime` 2.0))
            (if _returnvalue_2
              (bind _asbp_player_character (cast `/Game/Dynamics/PlayerCharacter/Blueprints/BP_PlayerCharacter` (`.HitActor` (`GameplayStatics.BreakHitResult` _outhit))))
              (if (`KismetSystemLibrary.IsValid` _asbp_player_character)
                (`GameplayStatics.ApplyDamage` _asbp_player_character 20.0))))
          (:`then_1`
            (`GameplayStatics.PlayWorldCameraShake` "/Game/Dynamics/BossFight/BP_AttackCameraShake.BP_AttackCameraShake_C" (`self.K2_GetActorLocation`) 0.0 1500.0)))))))

(event `self.Sphere.OnComponentBeginOverlap`
  (params (OverlappedComponent :type "PrimitiveComponent Object Reference") (OtherActor :type "Actor Object Reference") (OtherComp :type "PrimitiveComponent Object Reference") (OtherBodyIndex :type Integer) (bFromSweep :type Boolean) (SweepResult :type "HitResult Structure (by ref)"))
  ;[1 0.9736 0] Stupid Way Of Looking At Player
  (`BlackboardComponent.SetValueAsBool` (`AIBlueprintHelperLibrary.GetBlackboard` null) "seeingTarget?" true)
  (`KismetSystemLibrary.K2_SetTimerDelegate` (delegate `Rotate`) 0.1 true)
  (`ActorComponent.K2_DestroyComponent` (`self.Sphere`)))

(event `Rotate`
  (bind (_returnvalue_roll _returnvalue_pitch _returnvalue_yaw) (`KismetMathLibrary.BreakRotator` (`KismetMathLibrary.RInterpTo` (`self.K2_GetActorRotation`) (`KismetMathLibrary.FindLookAtRotation` (`self.K2_GetActorLocation`) (`self.K2_GetActorLocation` (`GameplayStatics.GetPlayerCharacter` 0))) (`GameplayStatics.GetWorldDeltaSeconds`))))
  ;[1 0.9736 0] Stupid Way Of Looking At Player
  (`self.K2_SetActorRotation` (`KismetMathLibrary.MakeRotator` 0.0 0.0 _returnvalue_yaw)))

(fn `UpdateBlackboardHP`
  (bind _asbp_ai_boss (cast `/Game/Dynamics/BossFight/BP_AI_Boss` (`self.GetController`))
    (:`then`
      (`BlackboardComponent.SetValueAsFloat` (`AIBlueprintHelperLibrary.GetBlackboard` _asbp_ai_boss) (`KismetStringLibrary.Conv_StringToName` "HealthPercentage") (/ (`self.CurrentHealth`) (`self.MaxHealth`))))
    (:`CastFailed`
      (`KismetSystemLibrary.PrintString` "Failed to cast boss AI" true true (struct :`R` 1.0 :`B` 0.049534 :`A` 1.0)))))

(fn `UpdateBossHealthBar`
  (`ProgressBar.SetPercent` (`/Game/Dynamics/Blueprints/WidgetBlueprints/WB_BossFightHealth.HealthBar` (`self.BossHealth`)) (/ (`self.CurrentHealth`) (`self.MaxHealth`))))

(fn `UserConstructionScript`)